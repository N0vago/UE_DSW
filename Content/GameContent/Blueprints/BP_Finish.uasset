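; BP_Finish is the level's finish trigger, a capsule that spins in place and ends the run when the player touches it.
; Tick accumulates an angle from RotationSpeed and applies it, wrapped to 360 degrees, as the capsule's relative yaw.
; On overlap with BP_FirstPersonCharacter it shows the mouse cursor and adds the WB_EndScreen widget to the viewport.
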(event `self.ReceiveTick`
  (params (DeltaSeconds :type "Float (single-precision)"))
  (bind _output_get (set `self.Angle` (+ (* DeltaSeconds (`self.RotationSpeed`)) (`self.Angle`))))
  (`SceneComponent.K2_SetRelativeRotation` (`self.Capsule`) (`KismetMathLibrary.MakeRotator` 0.0 0.0 (mod _output_get 360.0)) false false))

(event `self.Capsule.OnComponentBeginOverlap`
  (params (OverlappedComponent :type "PrimitiveComponent Object Reference") (OtherActor :type "Actor Object Reference") (OtherComp :type "PrimitiveComponent Object Reference") (OtherBodyIndex :type Integer) (bFromSweep :type Boolean) (SweepResult :type "HitResult Structure (by ref)"))
  (cast `/Game/TemplateContent/FirstPerson/Blueprints/BP_FirstPersonCharacter` OtherActor)
  (set `PlayerController.bShowMouseCursor` true (`GameplayStatics.GetPlayerController` 0))
  (bind _returnvalue (`|CreateWidget` "/Game/GameContent/Blueprints/WB_EndScreen.WB_EndScreen_C"))
  (`UserWidget.AddToViewport` _returnvalue 0))

(fn `UserConstructionScript`)