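; BP_Button is a shootable button that runs a cube colour-sequence puzzle on a Door.
; A projectile hit starts the Door's sequence, disabling button collision until the OnSequenceEnd dispatcher re-enables it.
; The next hit checks the attempt, destroying both Door and button on success or resetting the button on failure.
; Its cube colour and text label show the current phase.
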(event `self.ReceiveBeginPlay`
  (`TextRenderComponent.K2_SetText` (`self.TextRender`) (`KismetTextLibrary.Conv_StringToText` "Start Sequence")))

(event `self.Cube.OnComponentHit`
  (params (HitComponent :type "PrimitiveComponent Object Reference") (OtherActor :type "Actor Object Reference") (OtherComp :type "PrimitiveComponent Object Reference") (NormalImpulse :type "Vector Structure") (Hit :type "HitResult Structure (by ref)"))
  (bind _door (`self.Door`))
  (bind _cube (`self.Cube`))
  (cast `/Game/TemplateContent/FirstPerson/Blueprints/BP_FirstPersonProjectile` OtherActor)
  (if (`self.IsSequenceEnd`)
    (bind _returnvalue (`Door.CheckAttempt` (`self.Door`)))
    (if _returnvalue
      (`self.K2_DestroyActor` (`self.Door`))
      (`self.K2_DestroyActor`)
      (else
        (set `self.IsSequenceEnd` false)
        (`TextRenderComponent.K2_SetText` (`self.TextRender`) (`KismetTextLibrary.Conv_StringToText` "Start Sequence"))
        (`MeshComponent.SetColorParameterValueOnMaterials` (`self.Cube`) "BaseColor" (struct :`R` 0.192751 :`G` 1.0 :`A` 1.0))))
    (else
      (`Door.StartCubeColorizeSequence` _door)
      (`MeshComponent.SetColorParameterValueOnMaterials` _cube "BaseColor" (struct :`R` 1.0 :`G` 0.897364 :`A` 1.0))
      (`TextRenderComponent.K2_SetText` (`self.TextRender`) (`KismetTextLibrary.Conv_StringToText` "Whait..."))
      (`PrimitiveComponent.SetCollisionEnabled` _cube "NoCollision")
      (add `Door.OnSequenceEnd` _door (delegate `OnSequenceEnd_Event`)))))

(event `OnSequenceEnd_Event`
  (`MeshComponent.SetColorParameterValueOnMaterials` (`self.Cube`) "BaseColor" (struct :`R` 1.0 :`A` 1.0))
  (`TextRenderComponent.K2_SetText` (`self.TextRender`) (`KismetTextLibrary.Conv_StringToText` "Check Attempt"))
  (set `self.IsSequenceEnd` true)
  (`PrimitiveComponent.SetCollisionEnabled` (`self.Cube`) "QueryAndPhysics"))

(fn `UserConstructionScript`)